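; Lobby game mode for the RTS game that tracks connected players, host map settings, character availability and start readiness.
; Logins and logouts update the player list, then EveryoneUpdate pushes player info, counts, available characters and kick entries to lobby controllers through interface messages.
; It also relays host setting changes, kicks and lobby shutdown for loading.
; ChangeCharacter possesses a new spectator pawn at the last PlayerStart, while SpawnPlayer is empty.
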(event Custom|StartLoadingScreen
  (for _array_element (Variables|Default|GetConnectedPlayersArray)
    (bind _out (Class|INTLobbyPc|LobbyPcRef(Message) _array_element))
    (Default|DisableLobby _out)))

(event Custom|HostUpdateGameSettings
  (params (SelectedMapImage :type Texture%202D%20Object%20Reference) (SelectedMapName :type Text) (SelectedMapTime :type Text))
  (Variables|Default|SetSelectedMapImage SelectedMapImage)
  (Variables|Default|SetSelectedMapName SelectedMapName)
  (Variables|Default|SetSelectedMapTime SelectedMapTime)
  (for _array_element (Variables|Default|GetConnectedPlayersArray)
    (bind _out (Class|INTLobbyPc|LobbyPcRef(Message) _array_element))
    (Default|UpdateLobbySetting _out (Variables|Default|GetSelectedMapName) (Variables|Default|GetSelectedMapTime) (Variables|Default|GetSelectedMapImage))))

(event Custom|PlayerKick
  (params (PlayerId :type Integer))
  ;[1 1 1] Kick
  (bind _out (Class|INTLobbyPc|LobbyPcRef(Message) (Utilities|Array|Get(acopy) (Variables|Default|GetConnectedPlayersArray) PlayerId)))
  (Default|Kicked _out))

(event Custom|SpawnPlayer
  (params (Player :type Player%20Controller%20Object%20Reference)))

(event Custom|EveryoneUpdate
  (bind _connectedplayersarray (Variables|Default|GetConnectedPlayersArray))
  (bind _output_get (Variables|Default|SetCurrentPlayer (Utilities|Array|Length (Variables|Default|GetConnectedPlayersArray))))
  (if (> _output_get 0)
    (Utilities|Array|Clear (Variables|Default|GetConnectedPlayersInfo))
    (for _array_element _connectedplayersarray
      (bind _out (Class|INTLobbyPc|LobbyPcRef(Message) _array_element))
      (Utilities|Array|AddUnique (Variables|Default|GetConnectedPlayersInfo) (Variables|/Game/RtsGame/Map/RtsPlayerController_Bp.RtsPlayerController_Bp_C|GetPlayerSetting _out))
      (Default|UpdateNumberOfPlayer _out (Variables|Default|GetCurrentPlayer) (Variables|Default|GetMaxPlayer)))
    (for _array_element_2 _connectedplayersarray
      (bind _out_2 (Class|INTLobbyPc|LobbyPcRef(Message) _array_element_2))
      (Default|AddPlayerInfo _out_2 (Variables|Default|GetConnectedPlayersInfo))
      (Default|UpdateAvailablesCharacters _out_2 (Variables|Default|GetAvailableCharacter))
      (CallFunction|AddKickList))
    (bind _array_element_3 (Utilities|Array|ForEachLoopwithBreak (Variables|Default|GetConnectedPlayersInfo))
      (:LoopBody
        (if (Utilities|Enum|Equal(Enum) (.PlayerCharacter (Utilities|Struct|BreakPlayerInfo _array_element_3)) "NewEnumerator2")
          (Variables|Default|SetCanWeStart false)
          (CallFunction|CannontStartGame)
          (else
            (Variables|Default|SetCanWeStart true)))))))

(event Custom|AddKickList
  (bind _out (Class|INTLobbyPc|LobbyPcRef(Message) (Game|GetPlayerController 0)))
  (Default|AddPlayertoKickWindow _out))

(event Custom|CannontStartGame
  (Utilities|Array|ForEachLoopwithBreak (Variables|Default|GetConnectedPlayersInfo)) ; enters at Break
)

(event Custom|ChangeCharacter
  (params (ConnectedPlayer :type Player%20Controller%20Object%20Reference) (CharacterClass :type RaceInfo%20Enum :default "NewEnumerator0") (ChangeStatus :type Boolean))
  (bind _spawnpoint (Variables|Default|GetSpawnPoint))
  (Development|PrintString "Hello")
  (if ChangeStatus
    (Development|PrintString "1")
    (Utilities|IsValid (Pawn|GetControlledPawn ConnectedPlayer)
      (:Is%20Valid
        (Actor|DestroyActor))
      (:Is%20Not%20Valid
        _))
    (bind _returnvalue (Game|SpawnActorfromClass "/Script/RtsGame.RtsSpectatorPawn" (Transformation|GetActorTransform (Utilities|Array|Get(acopy) _spawnpoint (- (Utilities|Array|Length _spawnpoint) 1))) "AlwaysSpawn" 0 0))
    (Pawn|Possess ConnectedPlayer _returnvalue)))

(event EventPostLogin
  (params (NewPlayer :type Player%20Controller%20Object%20Reference))
  (bind _output_get (Variables|Default|SetConnectedPlayer NewPlayer))
  (Utilities|Array|AddUnique (Variables|Default|GetConnectedPlayersArray) _output_get)
  (bind _outactors (Actor|GetAllActorsOfClass "/Script/Engine.PlayerStart"))
  (Variables|Default|SetSpawnPoint _outactors)
  (bind _gameinstance (Class|BPIGameInstance|GameInstanceRef(Message) (Game|GetGameInstance)))
  (Variables|Default|SetServerName (Variables|/Game/RtsGame/Menu/GameInstanceMenu.GameInstanceMenu_C|GetServerName _gameinstance))
  (Variables|Default|SetMaxPlayer (Variables|/Game/RtsGame/Menu/GameInstanceMenu.GameInstanceMenu_C|GetMaxPlayers _gameinstance))
  (bind _out (Class|INTLobbyPc|LobbyPcRef(Message) (Variables|Default|GetConnectedPlayer)))
  (Default|InitialSetup _out)
  (Default|SetupLobbyMenu _out (Variables|Default|GetServerName))
  (Default|UpdateLobbySetting _out (Variables|Default|GetSelectedMapName) (Variables|Default|GetSelectedMapTime) (Variables|Default|GetSelectedMapImage))
  (CallFunction|EveryoneUpdate)
  (CallFunction|SpawnPlayer (Variables|Default|GetConnectedPlayer)))

(event EventOnLogout
  (params (ExitingController :type Controller%20Object%20Reference))
  (bind _connectedplayersarray (Variables|Default|GetConnectedPlayersArray))
  (bind (_array_element _array_index) (Utilities|Array|ForEachLoopwithBreak _connectedplayersarray :!label _label)
    (:LoopBody
      (if (== _array_element ExitingController)
        (goto _label Break)))
    (:Completed
      (bind _out (Class|INTLobbyPc|LobbyPcRef(Message) (Utilities|Array|Get(acopy) _connectedplayersarray _array_index)))
      (Utilities|Array|SetArrayElem (Variables|Default|GetAvailableCharacter) (Variables|/Game/RtsGame/Map/RtsPlayerController_Bp.RtsPlayerController_Bp_C|GetSelectedCharacter _out) false)
      (Utilities|Array|RemoveIndex (Variables|Default|GetConnectedPlayersArray) _array_index)
      (Utilities|Array|RemoveIndex (Variables|Default|GetConnectedPlayersInfo) _array_index)
      (CallFunction|EveryoneUpdate))))

(fn ConstructionScript)

(fn LobbyGmRef
  (return self))