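; RTS map game mode Blueprint that handles player logins, apparently with partly wired lobby logic.
; On PostLogin it records the new controller in a unique Players list, gathers all PlayerStart actors as spawn points and reads the server name from the game instance.
; The max-player read, lobby controller setup and SpawnPlayer call are disconnected and never run.
; SpawnPlayer itself is an empty event, so no custom spawning happens here.
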(event Custom|SpawnPlayer
  (params (Player :type Player%20Controller%20Object%20Reference)))

(event EventPostLogin
  (params (NewPlayer :type Player%20Controller%20Object%20Reference))
  (bind _output_get (Variables|Default|SetConnectedPlayer NewPlayer))
  (Utilities|Array|AddUnique (Variables|Default|GetPlayers) _output_get)
  (bind _outactors (Actor|GetAllActorsOfClass "/Script/Engine.PlayerStart"))
  (Variables|Default|SetSpawnPoint _outactors)
  (bind _gameinstance (Class|BPIGameInstance|GameInstanceRef(Message) (Game|GetGameInstance)))
  (Variables|Default|SetServerName (Variables|/Game/RtsGame/Menu/GameInstanceMenu.GameInstanceMenu_C|GetServerName _gameinstance)))

(fn ConstructionScript)