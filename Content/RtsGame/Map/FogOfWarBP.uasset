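; Fog of war Blueprint that maintains the FogOfWar render target for the RTS map.
; On BeginPlay it creates a dynamic instance of M_SubtractionFogOfWar and clears the render target to opaque black.
; SubtractFromFog sets the material's draw location and size from its inputs, then draws it onto the render target to carve out revealed areas.
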(event Custom|SubtractFromFog
  (params (VectorConversion :type Vector%202D%20Structure) (Value :type Float%20%28single-precision%29))
  (Rendering|Material|SetVectorParameterValue (Variables|Default|GetFogSubsraction) "DrawLocation" (Math|Conversions|ToLinearColor(Vector) (Math|Conversions|ToVector(Vector2D) VectorConversion)) :!class /Script/Engine.MaterialInstanceDynamic)
  (Rendering|Material|SetScalarParameterValue (Variables|Default|GetFogSubsraction) "DrawSize" Value :!class /Script/Engine.MaterialInstanceDynamic)
  (Rendering|DrawMaterialtoRenderTarget "/Game/RtsGame/Map/Textures/FogOfWar.FogOfWar" (Variables|Default|GetFogSubsraction)))

(event EventBeginPlay
  (bind _returnvalue (Rendering|Material|CreateDynamicMaterialInstance "/Game/RtsGame/Map/Materials/M_SubtractionFogOfWar.M_SubtractionFogOfWar" "None" :!class /Script/Engine.KismetMaterialLibrary))
  (Variables|Default|SetFogSubsraction _returnvalue)
  (Rendering|ClearRenderTarget2D "/Game/RtsGame/Map/Textures/FogOfWar.FogOfWar"))

(fn ConstructionScript)